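; Two-sided traffic light that endlessly alternates green and red between its sides, with a shared amber phase before each switch.
; BeginPlay loops through the Side2Green and Side1Green events on timed delays, and each event swaps on/off materials on the lamp components.
; Separately, StartFload waits a random sub-second delay, then ping-pongs the Cube's relative location forever using two chained timelines, one played forward and one reversed.
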(event `Side1Green`
  (`KismetSystemLibrary.Delay` 5.0)
  (`PrimitiveComponent.SetMaterial` (`self.Amber1`) 0 "/Game/Materials/Traffic_Light/Amber_ON.Amber_ON")
  (`PrimitiveComponent.SetMaterial` (`self.Amber2`) 0 "/Game/Materials/Traffic_Light/Amber_ON.Amber_ON")
  (`PrimitiveComponent.SetMaterial` (`self.Green2`) 0 "/Game/Materials/Traffic_Light/Green_Off.Green_Off")
  (`KismetSystemLibrary.Delay` 5.0)
  (`PrimitiveComponent.SetMaterial` (`self.Amber1`) 0 "/Game/Materials/Traffic_Light/Amber_Off.Amber_Off")
  (`PrimitiveComponent.SetMaterial` (`self.Amber2`) 0 "/Game/Materials/Traffic_Light/Amber_Off.Amber_Off")
  (`PrimitiveComponent.SetMaterial` (`self.Green1`) 0 "/Game/Materials/Traffic_Light/Green_ON.Green_ON")
  (`PrimitiveComponent.SetMaterial` (`self.Red2`) 0 "/Game/Materials/Traffic_Light/Red_ON.Red_ON")
  (`PrimitiveComponent.SetMaterial` (`self.Red1`) 0 "/Game/Materials/Traffic_Light/Red_Off.Red_Off"))

(event `self.ReceiveBeginPlay`
  (`self.Start Fload`)
  (`self.Side2Green` :!label _label)
  (`KismetSystemLibrary.Delay` 10.0)
  (`self.Side1Green`)
  (`KismetSystemLibrary.Delay` 10.0)
  (if true
    (goto _label)))

(event `Side2Green`
  (`KismetSystemLibrary.Delay` 5.0)
  (`PrimitiveComponent.SetMaterial` (`self.Amber1`) 0 "/Game/Materials/Traffic_Light/Amber_ON.Amber_ON")
  (`PrimitiveComponent.SetMaterial` (`self.Amber2`) 0 "/Game/Materials/Traffic_Light/Amber_ON.Amber_ON")
  (`PrimitiveComponent.SetMaterial` (`self.Green1`) 0 "/Game/Materials/Traffic_Light/Green_Off.Green_Off")
  (`KismetSystemLibrary.Delay` 5.0)
  (`PrimitiveComponent.SetMaterial` (`self.Amber1`) 0 "/Game/Materials/Traffic_Light/Amber_Off.Amber_Off")
  (`PrimitiveComponent.SetMaterial` (`self.Amber2`) 0 "/Game/Materials/Traffic_Light/Amber_Off.Amber_Off")
  (`PrimitiveComponent.SetMaterial` (`self.Green2`) 0 "/Game/Materials/Traffic_Light/Green_ON.Green_ON")
  (`PrimitiveComponent.SetMaterial` (`self.Red1`) 0 "/Game/Materials/Traffic_Light/Red_ON.Red_ON")
  (`PrimitiveComponent.SetMaterial` (`self.Red2`) 0 "/Game/Materials/Traffic_Light/Red_Off.Red_Off"))

(event `Start Fload`
  (`KismetSystemLibrary.Delay` (`KismetMathLibrary.RandomFloatInRange` 0.0 1.0))
  (bind (_direction _newtrack_0) (`Timeline|Timeline` :!via `PlayFromStart` :!label _label_2)
    (:`Update`
      (`SceneComponent.K2_SetRelativeLocation` (`self.Cube`) _newtrack_0 false false))
    (:`Finished`
      (bind (_direction_2 _newtrack_0_2) (`Timeline|Timeline_0` :!via `ReverseFromEnd`)
        (:`Update`
          (`SceneComponent.K2_SetRelativeLocation` (`self.Cube`) _newtrack_0_2 false false))
        (:`Finished`
          (goto _label_2 :!via `PlayFromStart`))))))

(fn `UserConstructionScript`)